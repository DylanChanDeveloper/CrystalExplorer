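; BP_PlayerPawn is the player pawn, moved by rolling its mesh with torque from the forward/back and left/right input axes.
; It fades the camera in on BeginPlay.
; The first damage it takes triggers Restart Level, which fades to black, waits, then reopens the current level.
; AdjustSpringArm sets the camera arm's length, yaw and pitch in world space, with no caller in this Blueprint.
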(event EventBeginPlay
  (CameraFades|StartCameraFade :self (Game|GetPlayerCameraManager 0) :FromAlpha 1.0 :Duration 3.0))

(event Collision|EventActorBeginOverlap
  (params (OtherActor :type Actor%20Object%20Reference)))

(event EventTick
  (params (DeltaSeconds :type Float%20%28single-precision%29)))

(event Collision|EventHit
  (params (MyComp :type Primitive%20Component%20Object%20Reference) (Other :type Actor%20Object%20Reference) (OtherComp :type Primitive%20Component%20Object%20Reference) (bSelfMoved :type Boolean) (HitLocation :type Vector :default "0, 0, 0") (HitNormal :type Vector :default "0, 0, 0") (NormalImpulse :type Vector :default "0, 0, 0") (Hit :type Hit%20Result%20Structure%20%28by%20ref%29)))

(event Game|Damage|EventAnyDamage
  (params (Damage :type Float%20%28single-precision%29) (DamageType :type Damage%20Type%20Object%20Reference) (InstigatedBy :type Controller%20Object%20Reference) (DamageCauser :type Actor%20Object%20Reference))
  (Utilities|FlowControl|DoOnce false
    (:Completed
      (Utilities|RestartLevel))))

(event Input|AxisEvents|InputAxisMoveForwards/Backwards
  (params (AxisValue :type Float%20%28single-precision%29))
  (Class|PrimitiveComponent|AddTorqueinRadians (Variables|Default|GetPlayerMesh) (Math|Vector|MakeVector 0.0 (* AxisValue (Variables|Default|GetSpeed%20multiplier)) 0.0) "None" true))

(event Input|AxisEvents|InputAxisMoveLeft/Right
  (params (AxisValue :type Float%20%28single-precision%29))
  (Class|PrimitiveComponent|AddTorqueinRadians (Variables|Default|GetPlayerMesh) (Math|Vector|MakeVector (* AxisValue (Variables|Default|GetSpeed%20multiplier)) 0.0 0.0) "None" true))

(fn ConstructionScript)

(fn AdjustSpringArm
  (params (Distance :type Float%20%28double-precision%29) (yaw :type Float%20%28double-precision%29) (pitch :type Float%20%28double-precision%29))
  (bind _springarm (Variables|Default|GetSpringArm))
  (Variables|/Script/Engine.SpringArmComponent|SetTargetArmLength _springarm Distance)
  (Transformation|SetWorldRotation _springarm (Math|Rotator|MakeRotator 0.0 pitch yaw) false false))