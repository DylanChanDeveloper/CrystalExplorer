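; BP_Cannon is a cannon actor that fires projectiles automatically in a repeating loop from BeginPlay.
; After a fire-rate delay, it spawns a BP_Projectiles actor at the spawn point's position and rotation, scaled by ProjectileScale.
; The CannonFiring timeline then animates the barrel along its local Y axis.
; The timeline's Cannon Fired event track restarts the delay, sustaining the loop without Tick.
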(event EventBeginPlay
  (Utilities|FlowControl|Delay (Variables|Cannonproperties|GetCannon%20fire%20rate) :!label _label)
  (CallFunction|SpawnProjectile)
  (bind _cannon_fire_animation (Timeline|Cannon%20Firing PlayFromStart)
    (:Update
      (CallFunction|MoveCannonBarrel _cannon_fire_animation))
    (:Cannon%20fired
      (goto _label))))

(event Collision|EventActorBeginOverlap
  (params (OtherActor :type Actor%20Object%20Reference)))

(event EventTick
  (params (DeltaSeconds :type Float%20%28single-precision%29)))

(fn ConstructionScript)

(fn SpawnProjectile
  (bind _projectile_spawn_point (Variables|Default|GetProjectile%20spawn%20point))
  (Game|SpawnActorfromClass "/Game/BluePrints/Actors/Projectiles/BP_Projectiles.BP_Projectiles_C" (Math|Transform|MakeTransform (Transformation|GetWorldLocation _projectile_spawn_point) (Transformation|GetWorldRotation _projectile_spawn_point) (Math|Conversions|ToVector(Float) (Variables|CannonProperties|GetProjectile%20scale))) "Undefined" 0 0))

(fn MoveCannonBarrel
  (params (Cannon%20barrel%20y%20location :type Float%20%28double-precision%29))
  (Transformation|SetRelativeLocation (Variables|Default|GetCannon%20Barrel) (Math|Vector|MakeVector 0.0 Cannon%20barrel%20y%20location 0.0) false false))