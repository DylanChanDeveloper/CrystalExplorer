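; BP_WinVolume is a volume that completes the level when the player overlaps it and every crystal has been collected.
; On player overlap it counts remaining BP_Crystal actors and prints a warning if any exist.
; Otherwise it finds the current level in the LevelNames array and opens the next entry, or quits the game on the final level.
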(event Collision|EventActorBeginOverlap
  (params (OtherActor :type Actor%20Object%20Reference))
  (Utilities|IsPlayer(macroLibarary) OtherActor
    (:Is%20Player
      (if (CallFunction|AnyCrystalRemaining)
        (Development|PrintString "Crystals still remaining" true true "(R=0.000000,G=0.660000,B=1.000000,A=1.000000)" 4.0)
        (else
          (levelmanagement|CompleteLevel))))))

(fn ConstructionScript)

(fn AnyCrystalRemaining
  (bind _outactors (Actor|GetAllActorsOfClass "/Game/BluePrints/Actors/Collectables/BP_Crystal.BP_Crystal_C"))
  (return (> (Utilities|Array|Length _outactors) 0)))

(fn GetNextLevelName
  (bind _result (Math|Integer|IncrementInt (LevelManagement|GetCurrentLevelIndex))
    (:%20%20
      (return (Utilities|Array|Get(acopy) (Variables|Default|GetLevel%20names) _result)))))

(fn LoadNextLevel
  (Game|OpenLevel(byName) (levelmanagement|GetNextLevelName)))

(fn IsFinalLevel?
  (return (== (Utilities|Array|LastIndex (Variables|Default|GetLevel%20names)) (LevelManagement|GetCurrentLevelIndex))))

(fn CompleteLevel
  (if (levelmanagement|IsFinalLevel?)
    (Game|QuitGame 0 "Quit" false)
    (else
      (levelmanagement|LoadNextLevel))))

(fn GetCurrentLevelIndex
  ;[1 1 1] Gets the current level name, then is converted to a integar. the find function is going to look through our level name array and try to find our current level name there and it will return the index.
  (bind _returnvalue (Game|GetCurrentLevelName true))
  (return (Utilities|Array|FindItem (Variables|Default|GetLevel%20names) (Utilities|String|StringToName _returnvalue))))